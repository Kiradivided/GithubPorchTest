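; Interactable door actor that swings open and closed each time its Interacted event fires.
; The event flips IsOpened and plays or reverses the RotationFacingX timeline, whose track drives the Door component's relative yaw.
; Tick stores delta time and prints IsOpened for debugging.
; A separate ToggleDoor function interpolates world rotation toward a target but is not called in this graph.
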(event `self.ReceiveTick`
  (params (DeltaSeconds :type "Float (single-precision)"))
  (set `self.Delta` DeltaSeconds)
  (`KismetSystemLibrary.PrintString` (`KismetStringLibrary.Conv_BoolToString` (`self.isOpened`)) true true (struct :`G` 0.66 :`B` 1.0 :`A` 1.0) 2.0 "DoorC"))

(event `/Game/FirstPerson/Blueprints/BPI_Interaction.Interacted`
  (if (`self.isOpened`)
    (set `self.isOpened` false)
    (bind (_direction _door_rotate) (`Timeline|RotationFacingX` :!via `Reverse` :!label _label)
      (:`Update`
        (`SceneComponent.K2_SetRelativeRotation` (`self.Door`) (`KismetMathLibrary.MakeRotator` 0.0 0.0 _door_rotate) false false)))
    (else
      (set `self.isOpened` true)
      (goto _label))))

(fn `Toggle Door`
  (params (DeltaTime :type "Float (single-precision)") (`Door Rot` :type "Rotator Structure"))
  (bind _door (`self.Door`))
  (`SceneComponent.K2_SetWorldRotation` _door (`KismetMathLibrary.RInterpTo` (`SceneComponent.K2_GetComponentRotation` _door) `Door Rot` DeltaTime 0.5) false false))

(fn `UserConstructionScript`)